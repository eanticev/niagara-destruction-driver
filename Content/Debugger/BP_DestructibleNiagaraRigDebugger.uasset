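; Debug actor that triggers destruction forces on Niagara destruction driver actors to test destructible rigs.
; A sphere, sized from Radius at BeginPlay and drawn every tick, initiates a destruction force at its location when it overlaps a driver actor.
; An unconnected manual path instead writes force center, radius, start time and duration straight to the driver's Niagara component, with debug output.
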(event `self.ReceiveBeginPlay`
  (`SphereComponent.SetSphereRadius` (`self.Sphere`) (`self.Radius`) true))

(event `self.ReceiveActorBeginOverlap`
  (params (OtherActor :type "Actor Object Reference"))
  (bind _asniagara_destruction_driver_actor (cast `NiagaraDestructionDriverActor` OtherActor))
  (`NiagaraDestructionDriverHelper.InitiateDestructionForce` (`self.K2_GetActorLocation`) (`SphereComponent.GetScaledSphereRadius` (`self.Sphere`))))

(event `self.ReceiveTick`
  (params (DeltaSeconds :type "Float (single-precision)"))
  (`KismetSystemLibrary.DrawDebugSphere` (`self.K2_GetActorLocation`) (`SphereComponent.GetScaledSphereRadius` (`self.Sphere`)) 12 (struct :`R` 1.0 :`G` 0.587542 :`B` 0.235882 :`A` 1.0)))

(fn `UserConstructionScript`)